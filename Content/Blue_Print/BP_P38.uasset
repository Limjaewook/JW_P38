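; BP_P38 is a P-38 aircraft actor that spins its two propellers and flies steadily in a straight line.
; Each Tick rolls the left and right propeller components about local X, using a separate speed variable for each.
; The same Tick moves the actor along world X at a fixed, frame-rate-independent speed, regardless of its facing.
; BeginPlay, overlap and construction logic are empty.
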(event EventBeginPlay)

(event Collision|EventActorBeginOverlap
  (params (OtherActor :type Actor%20Object%20Reference)))

(event EventTick
  (params (DeltaSeconds :type Float%20%28single-precision%29))
  (Variables|Default|SetDelta%20Seconds DeltaSeconds)
  ;[1 1 1] 왼쪽 프로펠러 회전
  (Transformation|AddLocalRotation (Variables|Default|GetL_PRO) (Math|Rotator|MakeRotator (* (Variables|Default|GetDelta%20Seconds) (Variables|Default|Getl_Propeller_Rotation_Speed)) 0.0 0.0) false false)
  ;[1 1 1] 오른쪽 프로펠러 회전
  (Transformation|AddLocalRotation (Variables|Default|GetR_PRO) (Math|Rotator|MakeRotator (* (Utilities|Time|GetWorldDeltaSeconds) (Variables|Default|GetR_Propeller_Rotation_Speed)) 0.0 0.0) false false)
  ;[1 1 1] 비행기전진
  (Transformation|AddActorWorldOffset self (Math|Vector|MakeVector (* (Utilities|Time|GetWorldDeltaSeconds) 3e+02) 0.0 0.0)))

(fn ConstructionScript)